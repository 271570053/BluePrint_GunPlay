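; BP_GameState is a game state Blueprint that indexes target locations and relays score changes to the VR player's shooter UI.
; On BeginPlay it maps every BP_TargetLocation actor in the level by TargetName.
; SetWidget finds the UI_Shooter on player 0's BP_VRPlayerBase widget component and binds UpdateWidget to the UpdateScore event.
; UpdateWidget then writes Score to that UI, so the display refreshes by event instead of on Tick.
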(event Custom|UpdateWidget
  ;[0.15 0.15 0.15 0.5] 更新分数
  (Default|SetScore (stale Custom|SetWidget _asui_shooter) (Utilities|Text|ToText(Integer) (Variables|Default|GetScore))))

(event Custom|SetWidget
  ;[0.15 0.15 0.15 0.5] 更新分数
  (bind _asbp_vrplayer_base (Utilities|Casting|CastToBP_VRPlayerBase (Game|Player|GetPlayerPawn 0)))
  (bind _asui_shooter (Utilities|Casting|CastToUI_Shooter (UserInterface|GetUserWidgetObject (Variables|/Game/Player/BP_VRPlayerBase.BP_VRPlayerBase_C|GetWidget _asbp_vrplayer_base))))
  (EventDispatchers|BindEventtoUpdateScore (delegate Custom|UpdateWidget)))

(event EventBeginPlay
  (bind _outactors (Actor|GetAllActorsOfClass "/Game/AI/Actor/BP_TargetLocation.BP_TargetLocation_C"))
  (for _array_element _outactors
    (Utilities|Map|Add (Variables|Default|GetTargetLocationMap) (Variables|/Game/AI/Actor/BP_TargetLocation.BP_TargetLocation_C|GetTargetName _array_element) _array_element)))

(event EventTick
  (params (DeltaSeconds :type Float%20%28single-precision%29)))

(fn ConstructionScript)