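; Game mode for gun play that turns players into bystanders and ends the session once every player has become one.
; The Bystander event destroys the controller's pawn, then spawns and possesses a BP_VRPlayerBase at the same transform.
; It counts each conversion, and when the count reaches the number of player controllers it calls EndSession for each of them.
; A QuitGame node is present but never runs.
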(event Custom|Bystander
  (params (PlayerController :type Controller%20Object%20Reference))
  (bind _output_get (Variables|Default|SetOldPawn (Pawn|GetControlledPawn PlayerController)))
  (bind _output_get_2 (Variables|Default|SetOldPawnTransform (Transformation|GetActorTransform _output_get)))
  (Pawn|UnPossess PlayerController)
  (Actor|DestroyActor (Variables|Default|GetOldPawn))
  (bind _returnvalue (Game|SpawnActorfromClass "/Game/Player/BP_VRPlayerBase.BP_VRPlayerBase_C" _output_get_2 "Undefined" "MultiplyWithRoot" 0 0))
  (Pawn|Possess PlayerController _returnvalue)
  (bind _output_get_3 (Variables|Default|SetNumOfBystander (+ (Variables|Default|GetNumOfBystander) 1)))
  (if (>= _output_get_3 (Class|GameplayStatics|GetNumPlayerControllers))
    (for _index (range 0 (- (Class|GameplayStatics|GetNumPlayerControllers) 1))
      (|EndSession (Game|GetPlayerController _index)))))

(event EventBeginPlay)

(event EventTick
  (params (DeltaSeconds :type Float%20%28single-precision%29)))

(fn ConstructionScript)