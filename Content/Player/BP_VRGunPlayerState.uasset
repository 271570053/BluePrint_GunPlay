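; BP_VRGunPlayerState is a VR gun player state that pushes score and health to the shooter UI.
; Both custom events take a target and cast the user widget in its Widget0 component to UI_Shooter.
; SetWidget displays PlayerScore as text, while UpDateBar checks the target is valid, then passes a percentage to the health bar.
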(event Custom|SetWidget
  (params (目标 :type BP%20VR%20Gun%20Player%20Object%20Reference))
  ;[0.15 0.15 0.15 0.5] 更新分数
  (bind _asui_shooter (Utilities|Casting|CastToUI_Shooter (UserInterface|GetUserWidgetObject (Variables|/Game/Player/BP_VRGunPlayer.BP_VRGunPlayer_C|GetWidget_0 目标))))
  (Default|SetScore _asui_shooter (Utilities|Text|ToText(Integer) (Variables|Default|GetPlayerScore))))

(event Custom|UpDateBar
  (params (目标 :type BP%20VR%20Gun%20Player%20Object%20Reference) (InPercent :type Float%20%28single-precision%29))
  (Utilities|IsValid 目标
    (:Is%20Valid
      (bind _asui_shooter (Utilities|Casting|CastToUI_Shooter (UserInterface|GetUserWidgetObject (Variables|/Game/Player/BP_VRGunPlayer.BP_VRGunPlayer_C|GetWidget_0 目标))))
      (Default|UpdateHealthBar _asui_shooter InPercent))))

(event EventBeginPlay)

(event EventTick
  (params (DeltaSeconds :type Float%20%28single-precision%29)))

(fn ConstructionScript)