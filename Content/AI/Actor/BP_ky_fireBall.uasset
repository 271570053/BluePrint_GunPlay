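; Fireball projectile actor that damages the VR player on contact.
; On spawn it emits a tinted shockwave particle, then flies along its local X axis with speed scaled by a timeline.
; Each tick a sphere trace ignoring GruxPlayerCharacter actors destroys it on any hit and calls HitPlayer.
; HitPlayer subtracts health from BP_VRPlayerBase, then updates the UI_Shooter health bar or quits the game at zero.
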(event EventBeginPlay
  (bind _defaultsceneroot (Variables|Default|GetDefaultSceneRoot))
  ;[1 1 1] Actor生成位置和冲击波颜色
  (bind _returnvalue (Effects|SpawnEmitteratLocation "/Game/FXVarietyPack/Particles/P_ky_shotShockwave.P_ky_shotShockwave" (Transformation|GetWorldLocation _defaultsceneroot) (Transformation|GetWorldRotation _defaultsceneroot)))
  (Effects|Components|ParticleSystem|SetVectorParameter _returnvalue "color" (Math|Conversions|ToVector(LinearColor) (Variables|Default|Getcolor)))
  ;[1 1 1] effect move correct
  (bind _valuecorrect (Timeline|Timeline_0 Play)
    (:Update
      (Variables|Default|SetspeedCorrect _valuecorrect))))

(event EventTick
  (params (DeltaSeconds :type Float%20%28single-precision%29))
  (bind _returnvalue (Transformation|GetActorLocation))
  ;[1 1 1] duration increment for control
  (Variables|Default|Setduration (- (Variables|Default|Getduration) DeltaSeconds))
  ;[1 1 1] move control
  (Transformation|AddActorLocalOffset (Math|Vector|MakeVector (* (Variables|Default|Getspeed) (Variables|Default|GetspeedCorrect) (Utilities|Time|GetWorldDeltaSeconds)) 0.0 0.0) false false)
  (bind _outactors (Actor|GetAllActorsOfClass "/Game/AI/BOSSAnimations/GruxPlayerCharacter.GruxPlayerCharacter_C"))
  (bind (_outhit _returnvalue_2) (Collision|SphereTraceForObjects _returnvalue _returnvalue 3e+01 (Variables|Default|GetCollisionObject) false _outactors "None"))
  (if _returnvalue_2
    (Actor|DestroyActor)
    ;[0.15 0.15 0.15 0.5] 玩家扣血
    (CallFunction|HitPlayer (.hitactor _outhit))))

(fn ConstructionScript)

(fn HitPlayer
  (params (Object :type Object%20Object%20Reference))
  (bind _asbp_vrplayer_base (Utilities|Casting|CastToBP_VRPlayerBase Object))
  (bind _asui_shooter (Utilities|Casting|CastToUI_Shooter (UserInterface|GetUserWidgetObject (Variables|/Game/Player/BP_VRPlayerBase.BP_VRPlayerBase_C|GetWidget _asbp_vrplayer_base))))
  (bind _output_get (Variables|/Game/Player/BP_VRPlayerBase.BP_VRPlayerBase_C|SetPlayerHP _asbp_vrplayer_base (- (Variables|/Game/Player/BP_VRPlayerBase.BP_VRPlayerBase_C|GetPlayerHP _asbp_vrplayer_base) 1e+01)))
  (if (== (Math|Float|Clamp(Float) (/ _output_get 1e+02)) 0.0)
    (Game|QuitGame 0 "Quit" false)
    (else
      (Default|UpdateHealthBar _asui_shooter (Math|Float|Clamp(Float) (/ _output_get 1e+02)))
      (Actor|DestroyActor))))