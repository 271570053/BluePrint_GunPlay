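; BP_FireBall is a fireball projectile that moves itself and reacts to players and walls.
; Each Tick it sweeps forward along local X by speed, a correction factor and delta time, then sphere-traces at its location, ignoring all GruxPlayerCharacter actors.
; A hit actor tagged Player is passed to HitPlayer, while any other hit destroys the fireball.
; The trace draws debug shapes every frame.
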(event EventBeginPlay
  (|CallParentFunction) ; 此节点被禁用，将不会被调用。\n从引脚连出引线来编译功能。
)

(event Collision|EventActorBeginOverlap
  (params (OtherActor :type Actor%20Object%20Reference)))

(event EventTick
  (params (DeltaSeconds :type Float%20%28single-precision%29))
  (bind _returnvalue (Transformation|GetActorLocation))
  ;[0.15 0.15 0.15 0.5] Tick移动位置
  (Transformation|AddActorLocalOffset (Math|Vector|MakeVector (* (Variables|Default|Getspeed) (Variables|Default|GetspeedCorrect) (Utilities|Time|GetWorldDeltaSeconds)) 0.0 0.0) true false)
  ;[0.15 0.15 0.15 0.5] 检测碰撞
  (bind _outactors (Actor|GetAllActorsOfClass "/Game/AI/BOSSAnimations/GruxPlayerCharacter.GruxPlayerCharacter_C"))
  (bind _outhit (Collision|SphereTraceForObjects _returnvalue _returnvalue 3e+01 (Variables|Default|GetCollisionObject) false _outactors "ForOneFrame"))
  (Utilities|IsValid (.hitactor _outhit)
    (:Is%20Valid
      (if (Actor|ActorHasTag (.hitactor _outhit) "Player")
        (CallFunction|HitPlayer (.hitactor _outhit))
        (else
          ;[0.15 0.15 0.15 0.5] 火球撞墙销毁
          (Actor|DestroyActor))))))

(fn ConstructionScript
  (|CallParentFunction))