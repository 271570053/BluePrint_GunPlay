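; BP_ky_explosion is an explosion actor that damages the VR gun player when caught in its radius.
; Every Tick it runs a sphere trace at its own location and casts the hit to BP_VRGunPlayer.
; It subtracts health directly from the player, then updates the player's UI_Shooter health bar and destroys itself, or quits the game if health reaches zero.
; It stays in the world until it hits the player.
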(event EventBeginPlay
  (|CallParentFunction) ; This node is disabled and will not be called.\nDrag off pins to build functionality.
)

(event Collision|EventActorBeginOverlap
  (params (OtherActor :type Actor%20Object%20Reference))
  (|CallParentFunction OtherActor) ; This node is disabled and will not be called.\nDrag off pins to build functionality.
)

(event EventTick
  (params (DeltaSeconds :type Float%20%28single-precision%29))
  (bind _returnvalue (Transformation|GetActorLocation))
  (bind _outhit (Collision|SphereTraceForObjects _returnvalue _returnvalue 1.5e+02 (Variables|Default|GetObject%20Types) false 0 "None"))
  (bind _asbp_vrgun_player (Utilities|Casting|CastToBP_VRGunPlayer (.hitactor _outhit)))
  ;[0.15 0.15 0.15 0.5] 伤害
  (bind _asui_shooter (Utilities|Casting|CastToUI_Shooter (UserInterface|GetUserWidgetObject (Variables|/Game/Player/BP_VRGunPlayer.BP_VRGunPlayer_C|GetWidget_0 _asbp_vrgun_player))))
  (bind _output_get (Variables|/Game/Player/BP_VRPlayerBase.BP_VRPlayerBase_C|SetPlayerHP _asbp_vrgun_player (- (Variables|/Game/Player/BP_VRPlayerBase.BP_VRPlayerBase_C|GetPlayerHP _asbp_vrgun_player) 1e+01)))
  (if (== (Math|Float|Clamp(Float) (/ _output_get 1e+02)) 0.0)
    (Game|QuitGame 0 "Quit" false)
    (else
      (Default|UpdateHealthBar _asui_shooter (Math|Float|Clamp(Float) (/ _output_get 1e+02)))
      (Actor|DestroyActor))))

(fn ConstructionScript
  (|CallParentFunction))