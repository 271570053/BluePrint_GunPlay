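; BP_Bullet is a projectile that damages zombies and the Grux boss when its sphere hits something.
; Hits on "Enemy"-tagged actors spawn blood and report damage to AI perception; other hits spawn a muzzle-flash effect, and the bullet destroys itself.
; Separate casts for zombie and boss feed shared logic that directly lowers clamped HP, destroys targets at zero, then increments the GameState score and updates its widget.
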(event OnComponentHit(Sphere)
  (params (HitComponent :type Primitive%20Component%20Object%20Reference) (OtherActor :type Actor%20Object%20Reference) (OtherComp :type Primitive%20Component%20Object%20Reference) (NormalImpulse :type Vector :default "0, 0, 0") (Hit :type Hit%20Result%20Structure%20%28by%20ref%29))
  (bind _returnvalue (Game|GetPlayerController 0))
  ;[0.15 0.15 0.15 0.5] 判断是否是敌人
  (if (Actor|ActorHasTag OtherActor "Enemy")
    (Utilities|FlowControl|Sequence
      (:then_0
        ;[0.15 0.15 0.15 0.5] 生成血水
        (Niagara|SpawnSystematLocation "/Game/MuzzleFlash/MuzzleFlash/Niagara/NS_Blood.NS_Blood" (.location Hit) "0, 0, 0" "2.000000,2.000000,2.000000"))
      (:then_1
        ;[0.15 0.15 0.15 0.5] Zombie分支
        ;;[0.15 0.15 0.15 0.5] 碰撞后就发送伤害事件给感官组件
        (bind _asbp_zombie_character_base (Utilities|Casting|CastToBP_ZombieCharacterBase OtherActor))
        (bind _output_get (Variables|Default|SetZombie _asbp_zombie_character_base))
        (Class|AISenseDamage|ReportDamageEvent _output_get _returnvalue 1e+01 "0, 0, 0" "0, 0, 0" "")
        ;;[0.15 0.15 0.15 0.5] 销毁子弹
        (Actor|DestroyActor :!label _label)
        (Utilities|IsValid (Variables|Default|GetZombie)
          (:Is%20Valid
            ;;[0.15 0.15 0.15 0.5] 更新血量
            (Variables|/Game/AI/BP_ZombieCharacterBase.BP_ZombieCharacterBase_C|SetHP (Variables|Default|GetZombie) (Math|Float|Clamp(Float) (- (Variables|/Game/AI/BP_ZombieCharacterBase.BP_ZombieCharacterBase_C|GetHP (Variables|Default|GetZombie)) 15.0) 0.0 1e+02))
            ;;[0.15 0.15 0.15 0.5] 0血销毁Actor
            (Development|PrintString (Utilities|String|ToString(Float) (Variables|/Game/AI/BP_ZombieCharacterBase.BP_ZombieCharacterBase_C|GetHP (Variables|Default|GetZombie))))
            (if (== (Variables|/Game/AI/BP_ZombieCharacterBase.BP_ZombieCharacterBase_C|GetHP (Variables|Default|GetZombie)) 0.0)
              (Actor|DestroyActor (Variables|Default|GetZombie))
              ;[0.15 0.15 0.15 0.5] 更新分数
              (bind _asbp_game_state (Utilities|Casting|CastToBP_GameState (Game|GetGameState) :!label _label_2))
              (Variables|/Game/ThirdPerson/Blueprints/BP_GameState.BP_GameState_C|SetScore _asbp_game_state (+ (Variables|/Game/ThirdPerson/Blueprints/BP_GameState.BP_GameState_C|GetScore _asbp_game_state) 1))
              (bind _asbp_game_state_2 (Utilities|Casting|CastToBP_GameState (Game|GetGameState)))
              (Default|UpdateWidget _asbp_game_state_2)))
          (:Is%20Not%20Valid
            ;[0.15 0.15 0.15 0.5] BOSS分支
            ;;[0.15 0.15 0.15 0.5] BOSS0血销毁BOSS
            (Variables|/Game/AI/BOSSAnimations/GruxPlayerCharacter.GruxPlayerCharacter_C|SetHP (Variables|Default|GetBOSS) (Math|Float|Clamp(Float) (- (Variables|/Game/AI/BOSSAnimations/GruxPlayerCharacter.GruxPlayerCharacter_C|GetHP (Variables|Default|GetBOSS)) 1e+01) 0.0 3e+03))
            (Development|PrintString (Utilities|String|ToString(Float) (Variables|/Game/AI/BOSSAnimations/GruxPlayerCharacter.GruxPlayerCharacter_C|GetHP (Variables|Default|GetBOSS))))
            (if (== (Variables|/Game/AI/BOSSAnimations/GruxPlayerCharacter.GruxPlayerCharacter_C|GetHP (Variables|Default|GetBOSS)) 0.0)
              (Actor|DestroyActor (Variables|Default|GetBOSS))
              (goto _label_2)))))
      (:then_2
        (bind _asgrux_player_character (Utilities|Casting|CastToGruxPlayerCharacter OtherActor))
        (bind _output_get_2 (Variables|Default|SetBOSS _asgrux_player_character))
        (Class|AISenseDamage|ReportDamageEvent _output_get_2 _returnvalue 1e+01 "0, 0, 0" "0, 0, 0" "")
        (goto _label)))
    (else
      ;[0.15 0.15 0.15 0.5] 不是敌人被击中生成火花
      (Utilities|FlowControl|Sequence
        (:then_0
          (Actor|DestroyActor))
        (:then_1
          (Niagara|SpawnSystematLocation "/Game/MuzzleFlash/MuzzleFlash/Niagara/NS_MuzzleFlash.NS_MuzzleFlash" (.location Hit)))))))

(event EventBeginPlay)

(event Collision|EventActorBeginOverlap
  (params (OtherActor :type Actor%20Object%20Reference)))

(event EventTick
  (params (DeltaSeconds :type Float%20%28single-precision%29)))

(fn ConstructionScript)