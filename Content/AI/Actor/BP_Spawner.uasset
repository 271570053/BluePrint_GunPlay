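; Server-side AI spawner that creates data-driven regular enemies and bosses when a BP_CollisionActor fires its spawn event with a matching SpawnID.
; On trigger it caches DTAIInfo rows and starts a timer, cleared after one SpawnActor pass.
; That pass reads DTSpawnInfo for count and class, spawns at random navigable points around itself, and sets stats plus blackboard speeds.
; A separate ID event sets SpawnID to the spawner count.
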(event Custom|ID
  ;[0.15 0.15 0.15 0.5] 手动设置ID
  (bind _outactors (Actor|GetAllActorsOfClass "BP_Spawner_C"))
  (Variables|Default|SetSpawnID (Utilities|Array|Length _outactors)))

(event Custom|自定义事件
  (params (NewParam :type Integer))
  (bind _dt_aiinfo (Variables|Default|GetDT_AIInfo))
  ;[0.15 0.15 0.15 0.5] 将表中属性存入二维数组
  (if (== NewParam (Variables|Default|GetSpawnID))
    (bind _outrownames (DataTable|GetDataTableRowNames _dt_aiinfo))
    (for _array_element _outrownames
      (bind _returnvalue (Utilities|GetDataTableRow _dt_aiinfo _array_element)
        (:then
          (Utilities|Array|Add (Variables|Default|GetAtttributeArray) _returnvalue))))
    (bind _returnvalue_2 (Utilities|Time|SetTimerbyFunctionName 0 "SpawnActor" (Variables|Default|GetSpawnTime) true))
    (Variables|Default|SetSpawnTimer _returnvalue_2)))

(event EventBeginPlay
  (Networking|SwitchHasAuthority
    (:Authority
      (bind _outactors (Actor|GetAllActorsOfClass "/Game/AI/Actor/BP_CollisionActor.BP_CollisionActor_C"))
      (for _array_element _outactors
        (EventDispatchers|BindEventtoSpawn _array_element (delegate Custom|自定义事件))))))

(event Collision|EventActorBeginOverlap
  (params (OtherActor :type Actor%20Object%20Reference)))

(event EventTick
  (params (DeltaSeconds :type Float%20%28single-precision%29)))

(fn ConstructionScript)

(fn SpawnActor
  (bind _returnvalue (Transformation|GetActorLocation))
  (bind _dt_spawninfo (Variables|Default|GetDT_SpawnInfo))
  (bind (_x _y _z) (Math|Vector|BreakVector _returnvalue))
  ;[0.15 0.15 0.15 0.5] 获取DT_Spawn信息
  (bind _outrownames (DataTable|GetDataTableRowNames _dt_spawninfo))
  (for _array_element _outrownames
    (bind _returnvalue_2 (Utilities|GetDataTableRow _dt_spawninfo _array_element)
      (:then
        ;[0.15 0.15 0.15 0.5] 根据SpawnID生成
        (if (== (Variables|Default|GetSpawnID) (.SpawnID (Utilities|Struct|BreakS_SpawnInfo _returnvalue_2)))
          ;[0.15 0.15 0.15 0.5] 控制生成数量
          (for _index (range 0 (- (.SpawnNum (Utilities|Struct|BreakS_SpawnInfo _returnvalue_2)) 1))
            ;[0.15 0.15 0.15 0.5] 根据Actor位置生成
            (bind _randomlocation (Class|NavigationSystemV1|GetRandomLocationinNavigableRadius (Math|Vector|MakeVector _x _y (+ _z 1e+02)) (Variables|Default|GetSpawnRadius) 0 0))
            ;[0.15 0.15 0.15 0.5] 如果是BOSS类就走这里
            (if (Utilities|IsValidClass (.BOSSBluePrint (Utilities|Struct|BreakS_AIAttribute (Utilities|Array|Get(acopy) (Variables|Default|GetAtttributeArray) (- (.AIClass (Utilities|Struct|BreakS_SpawnInfo _returnvalue_2)) 1)))))
              (bind _returnvalue_3 (Game|SpawnActorfromClass (.BOSSBluePrint (Utilities|Struct|BreakS_AIAttribute (Utilities|Array|Get(acopy) (Variables|Default|GetAtttributeArray) (- (.AIClass (Utilities|Struct|BreakS_SpawnInfo _returnvalue_2)) 1)))) (Math|Conversions|ToTransform(Vector) _randomlocation) "AdjustIfPossibleButAlwaysSpawn" "MultiplyWithRoot" 0 0))
              (Variables|/Game/AI/BOSSAnimations/GruxPlayerCharacter.GruxPlayerCharacter_C|SetHP _returnvalue_3 (.AIHP (Utilities|Struct|BreakS_AIAttribute (Utilities|Array|Get(acopy) (Variables|Default|GetAtttributeArray) (- (.AIClass (Utilities|Struct|BreakS_SpawnInfo _returnvalue_2)) 1)))))
              (AI|Components|Blackboard|SetValueasFloat (AI|GetBlackboard (AI|GetAIController _returnvalue_3)) (Variables|Default|GetBOSSChaseSpeed) (.ChaseSpeed (Utilities|Struct|BreakS_AIAttribute (Utilities|Array|Get(acopy) (Variables|Default|GetAtttributeArray) (- (.AIClass (Utilities|Struct|BreakS_SpawnInfo _returnvalue_2)) 1)))))
              (else
                ;[0.15 0.15 0.15 0.5] 生成普通小怪（缺点只能生成一个同一个基类）
                (bind _returnvalue_4 (Game|SpawnActorfromClass (.AIBluePrint (Utilities|Struct|BreakS_AIAttribute (Utilities|Array|Get(acopy) (Variables|Default|GetAtttributeArray) (- (.AIClass (Utilities|Struct|BreakS_SpawnInfo _returnvalue_2)) 1)))) (Math|Conversions|ToTransform(Vector) _randomlocation) "AdjustIfPossibleButAlwaysSpawn" "MultiplyWithRoot" 0 0))
                ;[0.15 0.15 0.15 0.5] 根据DT_Spawn中所需生成敌人属性设置
                (Variables|/Game/AI/BP_ZombieCharacterBase.BP_ZombieCharacterBase_C|SetHP _returnvalue_4 (.AIHP (Utilities|Struct|BreakS_AIAttribute (Utilities|Array|Get(acopy) (Variables|Default|GetAtttributeArray) (- (.AIClass (Utilities|Struct|BreakS_SpawnInfo _returnvalue_2)) 1)))))
                (Variables|/Game/AI/BP_ZombieCharacterBase.BP_ZombieCharacterBase_C|SetArmor _returnvalue_4 (.Armor (Utilities|Struct|BreakS_AIAttribute (Utilities|Array|Get(acopy) (Variables|Default|GetAtttributeArray) (- (.AIClass (Utilities|Struct|BreakS_SpawnInfo _returnvalue_2)) 1)))))
                ;[0.15 0.15 0.15 0.5] 用于匹配攻击动画
                (Variables|/Game/AI/BP_ZombieCharacterBase.BP_ZombieCharacterBase_C|SetAIClass _returnvalue_4 (.AIClass (Utilities|Struct|BreakS_SpawnInfo _returnvalue_2)))
                ;[0.15 0.15 0.15 0.5] 通过黑板键设置不同类型AI的追击/巡逻速度
                (AI|Components|Blackboard|SetValueasFloat (AI|GetBlackboard (AI|GetAIController _returnvalue_4)) (Variables|Default|GetChaseSpeed) (.ChaseSpeed (Utilities|Struct|BreakS_AIAttribute (Utilities|Array|Get(acopy) (Variables|Default|GetAtttributeArray) (- (.AIClass (Utilities|Struct|BreakS_SpawnInfo _returnvalue_2)) 1)))))
                (AI|Components|Blackboard|SetValueasFloat (AI|GetBlackboard (AI|GetAIController _returnvalue_4)) (Variables|Default|GetPatrolSpeed) (.PatrolSpeed (Utilities|Struct|BreakS_AIAttribute (Utilities|Array|Get(acopy) (Variables|Default|GetAtttributeArray) (- (.AIClass (Utilities|Struct|BreakS_SpawnInfo _returnvalue_2)) 1))))))))))))
  (Utilities|Time|ClearandInvalidateTimerbyHandle (Variables|Default|GetSpawnTimer)))