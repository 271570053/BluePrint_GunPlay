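; Base zombie AI character for a VR shooter, feeding its AI blackboard and detecting hand and head overlaps.
; Tick writes 2D player distance to the blackboard; capsule hits between zombies set own IsPatrol false if both patrol, otherwise true.
; Overlaps call UpdatePlayerHP, but its damage, health-bar and quit-at-zero logic is disconnected, so it does nothing.
; UpdateWalkSpeed exposes a setter for maximum walk speed.
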(event OnComponentBeginOverlap(HandCollision)
  (params (OverlappedComponent :type Primitive%20Component%20Object%20Reference) (OtherActor :type Actor%20Object%20Reference) (OtherComp :type Primitive%20Component%20Object%20Reference) (OtherBodyIndex :type Integer) (bFromSweep :type Boolean) (SweepResult :type Hit%20Result%20Structure%20%28by%20ref%29))
  ;[0.15 0.15 0.15 0.5] 玩家被攻击后减少血量
  (CallFunction|UpdatePlayerHP OtherActor))

(event OnComponentBeginOverlap(HeadCollision)
  (params (OverlappedComponent :type Primitive%20Component%20Object%20Reference) (OtherActor :type Actor%20Object%20Reference) (OtherComp :type Primitive%20Component%20Object%20Reference) (OtherBodyIndex :type Integer) (bFromSweep :type Boolean) (SweepResult :type Hit%20Result%20Structure%20%28by%20ref%29))
  ;[0.15 0.15 0.15 0.5] 玩家被攻击后减少血量
  (CallFunction|UpdatePlayerHP OtherActor))

(event OnComponentHit(CapsuleComponent)
  (params (HitComponent :type Primitive%20Component%20Object%20Reference) (OtherActor :type Actor%20Object%20Reference) (OtherComp :type Primitive%20Component%20Object%20Reference) (NormalImpulse :type Vector :default "0, 0, 0") (Hit :type Hit%20Result%20Structure%20%28by%20ref%29))
  (bind _self self)
  (bind _ispatrol (Variables|Default|GetIsPatrol))
  (bind _ispatrol_2 (Variables|Default|GetIsPatrol))
  (bind _returnvalue (AI|GetAIController _self))
  (bind _returnvalue_2 (AI|GetBlackboard _returnvalue))
  ;[0.15 0.15 0.15 0.5] 碰撞之后就更新黑板键
  (bind _asbp_zombie_character_base (Utilities|Casting|CastToBP_ZombieCharacterBase OtherActor))
  (Utilities|IsValid _asbp_zombie_character_base
    (:Is%20Valid
      (if (== (and (ScalableFloat|GetValueasBool (AI|GetBlackboard (AI|GetAIController _asbp_zombie_character_base)) _ispatrol_2) (ScalableFloat|GetValueasBool _returnvalue_2 _ispatrol_2)) true)
        (AI|Components|Blackboard|SetValueasBool _returnvalue_2 _ispatrol false)
        (else
          ;;[0.15 0.15 0.15 0.5] 都为false或者falseAndtrue就将false更新为true
          (AI|Components|Blackboard|SetValueasBool _returnvalue_2 _ispatrol true))))))

(event EventBeginPlay)

(event EventTick
  (params (DeltaSeconds :type Float%20%28single-precision%29))
  ;[0.15 0.15 0.15 0.5] 每Tick计算AI与玩家之间距离
  (AI|Components|Blackboard|SetValueasFloat (AI|GetBlackboard (AI|GetAIController self)) (Variables|Default|GetDistanceToPlayer) (Math|Vector|Distance2D(Vector) (Transformation|GetActorLocation) (Transformation|GetActorLocation (Game|Player|GetPlayerPawn 0)))))

(fn ConstructionScript)

(fn UpdateWalkSpeed
  (params (NewWalkSpeed :type Float%20%28double-precision%29))
  (Variables|/Script/Engine.CharacterMovementComponent|SetMaxWalkSpeed (Variables|Character|GetCharacterMovement) NewWalkSpeed))

(fn UpdatePlayerHP
  (params (Object :type Object%20Object%20Reference)))