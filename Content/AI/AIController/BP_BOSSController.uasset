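; BP_BOSSController is the boss's AI controller, which runs BT_BOSSBehaviorTree when it possesses a pawn.
; On perception updates, it adds BP_VRGunPlayer actors tagged "Player" to PlayerArray without duplicates, then removes invalid entries inside the loop over that array.
; The Blackboard write to PlayerKey is disconnected, so this graph does not pass detected players to the behavior tree.
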(event OnTargetPerceptionUpdated(AIPerception)
  (params (Actor :type Actor%20Object%20Reference) (Stimulus :type AI%20Stimulus%20Structure))
  (bind _playerarray (Variables|Default|GetPlayerArray))
  ;[0.15 0.15 0.15 0.5] 更新黑板键
  (Utilities|Casting|CastToBP_VRGunPlayer Actor)
  (if (Actor|ActorHasTag Actor "Player")
    (Utilities|Array|AddUnique _playerarray Actor)
    (for (_array_element _array_index) _playerarray
      (Utilities|IsValid _array_element
        (:Is%20Not%20Valid
          (Utilities|Array|RemoveIndex _playerarray _array_index))))))

(event EventBeginPlay)

(event EventPossess
  (params (PossessedPawn :type Pawn%20Object%20Reference))
  ;[0.15 0.15 0.15 0.5] 激活行为树
  (AI|RunBehaviorTree "/Game/AI/BOSSBehaviorTree/BT_BOSSBehaviorTree.BT_BOSSBehaviorTree"))

(fn ConstructionScript)