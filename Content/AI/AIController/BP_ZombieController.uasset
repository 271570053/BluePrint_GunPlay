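; BP_ZombieController is the AI controller for zombies, running the BT_AI behavior tree when it possesses a pawn.
; Each tick it writes the Player's location to the PlayerLocation blackboard key if that reference is valid, though these graphs never assign it.
; Successful perception stimuli, noted as damage sensing, store the sensed actor in TargetActor, which is never cleared here.
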(event OnTargetPerceptionUpdated(AIPerception)
  (params (Actor :type Actor%20Object%20Reference) (Stimulus :type AI%20Stimulus%20Structure))
  ;[0.15 0.15 0.15 0.5] 如果伤害感官触发就更新黑板键
  (if (.bSuccessfullySensed (Utilities|Struct|BreakAIStimulus Stimulus))
    (AI|Components|Blackboard|SetValueasObject (Variables|Default|GetBlackboard) (Variables|Default|GetTargetActor) Actor)))

(event EventBeginPlay)

(event EventPossess
  (params (PossessedPawn :type Pawn%20Object%20Reference))
  ;[0.15 0.15 0.15 0.5] 激活行为树
  (AI|RunBehaviorTree "/Game/AI/ZombieBehaviorTree/BT_AI.BT_AI"))

(event EventTick
  (params (DeltaSeconds :type Float%20%28single-precision%29))
  (bind _player (Variables|Default|GetPlayer))
  (Utilities|IsValid _player
    (:Is%20Valid
      (AI|Components|Blackboard|SetValueasVector (Variables|Default|GetBlackboard) (Variables|Default|GetPlayerLocation) (Transformation|GetActorLocation _player)))))

(fn ConstructionScript)