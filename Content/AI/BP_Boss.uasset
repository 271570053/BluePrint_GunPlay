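; BP_Boss is an AI boss Blueprint whose own logic is a single function for damaging the VR player.
; UpdateHP casts the passed object to BP_VRPlayerBase, subtracts a fixed amount from PlayerHP, and fetches the UI_Shooter from the player's widget component.
; It passes the clamped health fraction to the health bar, or quits the game outright when that reaches zero.
; BeginPlay and overlap events are unused stubs.
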(event EventBeginPlay)

(event Collision|EventActorBeginOverlap
  (params (OtherActor :type Actor%20Object%20Reference)))

(fn ConstructionScript
  (|CallParentFunction))

(fn UpdateHP
  (params (Object :type Object%20Object%20Reference))
  (bind _asbp_vrplayer_base (Utilities|Casting|CastToBP_VRPlayerBase Object))
  (bind _output_get (Variables|/Game/Player/BP_VRPlayerBase.BP_VRPlayerBase_C|SetPlayerHP _asbp_vrplayer_base (- (Variables|/Game/Player/BP_VRPlayerBase.BP_VRPlayerBase_C|GetPlayerHP _asbp_vrplayer_base) 1e+01)))
  (bind _asui_shooter (Utilities|Casting|CastToUI_Shooter (UserInterface|GetUserWidgetObject (Variables|/Game/Player/BP_VRPlayerBase.BP_VRPlayerBase_C|GetWidget _asbp_vrplayer_base))))
  (if (== (Math|Float|Clamp(Float) (/ _output_get 1e+02)) 0.0)
    (Game|QuitGame 0 "Quit" false)
    (else
      (Default|UpdateHealthBar _asui_shooter (Math|Float|Clamp(Float) (/ _output_get 1e+02))))))